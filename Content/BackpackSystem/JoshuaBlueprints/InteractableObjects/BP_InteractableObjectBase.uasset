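; Base interactable object for the backpack system that can be looked at, selected, picked up and dropped.
; Looking at it toggles an outline-style custom depth highlight and a mesh-centred particle effect unless already interacted with.
; Pickup disables physics and snaps it to a given component, while Drop detaches it and animates back toward its BeginPlay transform.
; Timelines and MoveComponentTo drive movement and scale changes, with collision disabled when transform moves start.
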(event OnComponentActivated(ParticleSystem)
  (params (Component :type Actor%20Component%20Object%20Reference) (bReset :type Boolean))
  (bind _staticmeshcomponent (Variables|Debug|GetStaticMeshComponent))
  (bind (_min _max) (Components|StaticMesh|GetLocalBounds _staticmeshcomponent))
  (bind (_x _y _z) (Math|Vector|BreakVector _max))
  (bind (_x_2 _y_2 _z_2) (Math|Vector|BreakVector _min))
  ;[1 1 1] Places the particle effect into the centre of the Static Mesh when its activated
  (Transformation|SetRelativeLocation (Variables|Default|GetParticleSystem) (Math|Vector|MakeVector (/ (+ _x_2 _x) 2.0) (/ (+ _y_2 _y) 2.0) (/ (+ _z_2 _z) 2.0)) false false))

(event Custom|MoveToWorldLocation
  (params (TargetLocation :type Vector))
  ;[1 1 1] Movement
  (bind _lerping (Timeline|LerpHalfSecond PlayFromStart)
    (:Update
      (Transformation|SetWorldLocation (Variables|Debug|GetStaticMeshComponent) (Math|Vector|Lerp(Vector) (Transformation|GetWorldLocation (Variables|Debug|GetStaticMeshComponent)) TargetLocation _lerping) false false))))

(event Custom|ChangeScale
  (params (From :type Vector) (To :type Vector))
  ;[1 1 1] Movement
  (bind _lerping (Timeline|HalfSecond PlayFromStart)
    (:Update
      (Transformation|SetRelativeScale3D (Variables|Debug|GetStaticMeshComponent) (Math|Vector|Lerp(Vector) From To _lerping)))))

(event Custom|Selected
  (params (Scale :type Vector))
  (bind _staticmeshcomponent (Variables|Debug|GetStaticMeshComponent))
  ;[1 1 1] Selected Object (From Backpack Select Function)
  (Utilities|FlowControl|Delay 0.4)
  (Rendering|SetRenderCustomDepth _staticmeshcomponent true)
  (Transformation|SetRelativeScale3D _staticmeshcomponent Scale))

(event Custom|MoveToTransform
  (params (Transform :type Transform))
  (bind (_location _rotation) (Math|Transform|BreakTransform Transform))
  (bind _staticmeshcomponent (Variables|Debug|GetStaticMeshComponent))
  ;[1 1 1] Movement
  (Collision|SetCollisionEnabled _staticmeshcomponent "NoCollision")
  (Components|MoveComponentTo _staticmeshcomponent _location _rotation false false 0.5 false)
  (Collision|SetCollisionEnabled _staticmeshcomponent "QueryAndPhysics"))

(event EventBeginPlay
  ;[1 1 1] BeginPlay
  (Variables|Default|SetOriginalTransform (Transformation|GetWorldTransform (Variables|Debug|GetStaticMeshComponent))))

(event EventPickup
  (params (AttachTo :type Scene%20Component%20Object%20Reference))
  ;[1 1 1] Grabbing and Releasing
  (Physics|SetSimulatePhysics (Variables|Debug|GetStaticMeshComponent) false)
  (Transformation|AttachComponentToComponent (VehicleSound|GetRootComponent) AttachTo "None" "SnapToTarget" "SnapToTarget" "KeepWorld" false))

(event EventDrop
  ;[1 1 1] Grabbing and Releasing
  (Transformation|DetachFromActor "KeepWorld" "KeepWorld" "KeepWorld")
  (CallFunction|MovetoTransform (Variables|Default|GetOriginalTransform)))

(event EventLookedat
  ;[1 1 1] Looked At Functions
  (if (not (Variables|Default|GetBeingInteractedWith))
    (Rendering|SetRenderCustomDepth (Variables|Debug|GetStaticMeshComponent) true)
    (Components|Activation|Activate (Variables|Default|GetParticleSystem) false)))

(event EventLookedAway
  ;[1 1 1] Looked At Functions
  (if (not (Variables|Default|GetBeingInteractedWith))
    (Rendering|SetRenderCustomDepth (Variables|Debug|GetStaticMeshComponent) false)
    (Components|Activation|Deactivate (Variables|Default|GetParticleSystem))))

(fn ConstructionScript)