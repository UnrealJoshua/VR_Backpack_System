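; Backpack inventory component for the motion-controller pawn that stores held interactable objects and displays them for selection.
; Stowing records the object's class and original transform, then destroys it.
; Opening respawns items in a camera-attached ring, normalized by mesh bounds; selection shifts the ring, enlarging and custom-depth highlighting the current item.
; Removal restores original scale; backpack mesh setup and stow-preview animation are unwired.
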(event Custom|BackpackButtonPressed
  (params (HeldActor :type Actor%20Object%20Reference))
  (bind _backpack_mesh (Variables|Default|GetBackpack%20Mesh))
  (bind _skeletalmeshcomponent (Variables|/Script/Engine.SkeletalMeshActor|GetSkeletalMeshComponent _backpack_mesh))
  (Utilities|IsValid HeldActor
    (:Is%20Valid
      (bind _asbp_interactable_object_base (Utilities|Casting|CastToBP_InteractableObjectBase HeldActor)
        (:then
          (CallFunction|PutinBackPack _asbp_interactable_object_base)
          ;[1 1 1] Needs to set the mesh, and scale
          (CallFunction|GoingIntoBackpackMesh)
          (Actor|DestroyActor _asbp_interactable_object_base))
        (:CastFailed
          (Development|PrintString "Must have Ineractable Objects going into backpack component!" true true "(R=1.000000,G=0.000000,B=0.015913,A=1.000000)"))))
    (:Is%20Not%20Valid
      (Development|PrintString "no actor held")
      (Rendering|SetVisibility (Variables|/Script/Engine.StaticMeshActor|GetStaticMeshComponent (Variables|Default|GetGoing%20into%20Backpack%20Mesh)) false false)
      (if (Variables|Default|GetBackpackOpen?)
        (CallFunction|HideBackpack)
        (Variables|Default|SetBackpack%20Play%20Rate 1.0)
        (Variables|Default|SetBackpackOpen? false)
        (else
          (CallFunction|ShowBackpack)
          (Variables|Default|SetBackpack%20Play%20Rate -1.0)
          (Variables|Default|SetBackpackOpen? true)))
      (Components|Timeline|SetPlayRate _skeletalmeshcomponent (Variables|Default|GetBackpack%20Play%20Rate))
      (Audio|Components|Audio|Play _skeletalmeshcomponent false)
      (Rendering|SetVisibility _skeletalmeshcomponent true false)
      (Utilities|FlowControl|RetriggerableDelay 1.0)
      (Rendering|SetVisibility (Variables|/Script/Engine.SkeletalMeshActor|GetSkeletalMeshComponent (Variables|Default|GetBackpack%20Mesh)) (Variables|Default|GetBackpackOpen?) false))))

(event Custom|GoingIntoBackpackMesh
  (bind _returnvalue (Game|SpawnActorfromClass "/Script/Engine.StaticMeshActor" (Math|Transform|MakeTransform "0, 0, 0") "Undefined" 0 0))
  (Variables|Default|SetGoing%20into%20Backpack%20Mesh _returnvalue)
  (Transformation|AttachComponentToComponent _returnvalue (Variables|Default|GetPlayerCamera) "None" "KeepRelative" "KeepRelative" "KeepRelative" true)
  (Transformation|SetActorRelativeTransform _returnvalue (Math|Transform|MakeTransform "30.000000,-10.000000,-10.000000" "0.000000,270.000000,0.000000" "0.010000,0.010000,0.010000") false false)
  (Collision|SetCollisionEnabled (Variables|/Script/Engine.StaticMeshActor|GetStaticMeshComponent _returnvalue) "NoCollision")
  (Variables|/Script/Engine.PrimitiveComponent|SetbGenerateOverlapEvents (Variables|/Script/Engine.StaticMeshActor|GetStaticMeshComponent _returnvalue) false)
  (Rendering|SetVisibility (Variables|/Script/Engine.StaticMeshActor|GetStaticMeshComponent _returnvalue) false false))

(event EventBeginPlay
  (bind _returnvalue (Components|GetOwner))
  (bind _returnvalue_2 (Actor|GetComponentbyClass _returnvalue "/Script/Engine.CameraComponent"))
  ;[1 1 1] TODO: Delete
  (Utilities|FlowControl|Sequence
    (:then_0
      (bind _asmotion_controller_pawn (Utilities|Casting|CastToMotionControllerPawn _returnvalue))
      (Variables|Default|SetMotionControllerPlayer _asmotion_controller_pawn))
    (:then_1
      (Utilities|IsValid (Variables|Default|GetPlayerCamera)
        (:Is%20Not%20Valid
          (Utilities|IsValid _returnvalue_2
            (:Is%20Valid
              (Variables|Default|SetPlayerCamera _returnvalue_2))
            (:Is%20Not%20Valid
              (Development|PrintString "Could not find camera on actor for backpack to attach to!" true true "(R=1.000000,G=0.000000,B=0.000000,A=1.000000)"))))))))

(fn PutinBackPack
  (params (Object :type BP%20Interactable%20Object%20Base%20Object%20Reference%20%28by%20ref%29))
  (bind _returnvalue (Utilities|Array|AddUnique (Variables|Default|GetOriginalTransformOfObjects) (Variables|/Game/BackpackSystem/JoshuaBlueprints/InteractableObjects/BP_InteractableObjectBase.BP_InteractableObjectBase_C|GetOriginalTransform Object)))
  (Utilities|Array|SetArrayElem (Variables|Default|GetStatic%20Objects%20in%20Backpack) _returnvalue (Utilities|GetClass Object) true))

(fn BackpackFull?
  (return (== (Variables|Default|GetBackPackSize) (Utilities|Array|Length (Variables|Default|GetStatic%20Objects%20in%20Backpack)))))

(fn RemoveCurrentItemfromBackpack
  (bind _arraypositioninteractingwith (Variables|Default|GetArrayPositionInteractingWith))
  (bind _arraypositioninteractingwith_2 (Variables|Default|GetArrayPositionInteractingWith))
  (bind _originaltransformofobjects (Variables|Default|GetOriginalTransformOfObjects))
  (Utilities|Array|RemoveIndex (Variables|Default|GetStatic%20Objects%20in%20Backpack) _arraypositioninteractingwith)
  (Utilities|Array|RemoveIndex (Variables|Default|GetStaticSpawnFromBackPack) _arraypositioninteractingwith)
  (Transformation|SetActorScale3D (Variables|Default|GetActorCurrentlyInteractingWith) (.Scale (Math|Transform|BreakTransform (Utilities|Array|Get(acopy) (Variables|Default|GetOriginalTransformOfObjects) _arraypositioninteractingwith))))
  (Rendering|SetRenderCustomDepth (Variables|/Script/Engine.StaticMeshActor|GetStaticMeshComponent (Variables|Default|GetActorCurrentlyInteractingWith)) false)
  (Variables|/Game/BackpackSystem/JoshuaBlueprints/InteractableObjects/BP_InteractableObjectBase.BP_InteractableObjectBase_C|SetOriginalTransform (Variables|Default|GetActorCurrentlyInteractingWith) (Utilities|Array|Get(acopy) _originaltransformofobjects _arraypositioninteractingwith_2))
  (Utilities|Array|RemoveIndex _originaltransformofobjects _arraypositioninteractingwith_2)
  (Variables|Default|SetActorCurrentlyInteractingWith 0))

(fn ShowBackpack
  (bind _static_objects_in_backpack (Variables|Default|GetStatic%20Objects%20in%20Backpack))
  (bind _staticspawnfrombackpack (Variables|Default|GetStaticSpawnFromBackPack))
  (bind _returnvalue (Utilities|Array|Length _staticspawnfrombackpack))
  (bind _returnvalue_2 (Utilities|Array|Length _staticspawnfrombackpack))
  (bind _returnvalue_3 (- _returnvalue_2 1))
  (if (not (== (Utilities|Array|Length (Variables|Default|GetStatic%20Objects%20in%20Backpack)) 0))
    (for (_ _array_index) _static_objects_in_backpack
      (bind _returnvalue_4 (Game|SpawnActorfromClass (Utilities|Array|Get(acopy) _static_objects_in_backpack _array_index) (Math|Transform|MakeTransform "0, 0, 0") "Undefined" 0 0))
      (Utilities|Array|Add (Variables|Default|GetStaticSpawnFromBackPack) _returnvalue_4)
      (if (Variables|Default|GetAttachToPlayer?)
        (Transformation|AttachComponentToComponent _returnvalue_4 (Variables|/Game/VirtualRealityBP/Blueprints/MotionControllerPawn.MotionControllerPawn_C|GetCamera (Variables|Default|GetMotionControllerPlayer)) "None" "KeepRelative" "KeepRelative" "KeepRelative" true)))
    (for (_array_element _array_index_2) _staticspawnfrombackpack
      (Transformation|SetActorRelativeTransform _array_element (Math|Transform|MakeTransform (Math|Vector|RotateVector (Math|Vector|MakeVector 45.0 0.0 12.0) (Math|Rotator|MakeRotator (* (- _array_index_2 (- _returnvalue 1)) (/ 3.6e+02 (Math|Conversions|ToFloat(Integer) _returnvalue))) 0.0 0.0)) (Math|Rotator|MakeRotator 0.0 0.0 9e+01) (CallFunction|GetSpawnSize _array_element)) false false))
    (Variables|Default|SetActorCurrentlyInteractingWith (Utilities|Array|Get(acopy) _staticspawnfrombackpack _returnvalue_3))
    (Rendering|SetRenderCustomDepth (Variables|/Script/Engine.StaticMeshActor|GetStaticMeshComponent (Variables|Default|GetActorCurrentlyInteractingWith)) true)
    (Transformation|SetRelativeScale3D (Variables|/Script/Engine.StaticMeshActor|GetStaticMeshComponent (Variables|Default|GetActorCurrentlyInteractingWith)) (* (CallFunction|GetSpawnSize _array_element) 2.0))
    (Variables|Default|SetArrayPositionInteractingWith _returnvalue_3)))

(fn HideBackpack
  (for _array_element (Variables|Default|GetStaticSpawnFromBackPack)
    (Actor|DestroyActor _array_element))
  (Utilities|Array|Clear (Variables|Default|GetStaticSpawnFromBackPack)))

(fn SelectItem
  (params (MoveRight? :type Boolean))
  (bind _staticspawnfrombackpack (Variables|Default|GetStaticSpawnFromBackPack))
  (bind _staticspawnfrombackpack_2 (Variables|Default|GetStaticSpawnFromBackPack))
  (bind _staticspawnfrombackpack_3 (Variables|Default|GetStaticSpawnFromBackPack))
  (bind _returnvalue (Utilities|Array|Length _staticspawnfrombackpack_3))
  (LocalVariables|SetMovingRight? MoveRight?)
  (Rendering|SetRenderCustomDepth (Variables|/Script/Engine.StaticMeshActor|GetStaticMeshComponent (Variables|Default|GetActorCurrentlyInteractingWith)) false)
  (Transformation|SetRelativeScale3D (Variables|/Script/Engine.StaticMeshActor|GetStaticMeshComponent (Variables|Default|GetActorCurrentlyInteractingWith)) (CallFunction|GetSpawnSize (Variables|Default|GetActorCurrentlyInteractingWith)))
  (if (LocalVariables|GetMovingRight?)
    (bind _result (Math|Integer|IncrementInt (Variables|Default|GetArrayPositionInteractingWith))
      (:%20%20
        (if (>= _result _returnvalue)
          (Variables|Default|SetArrayPositionInteractingWith 0))
        (Variables|Default|SetActorCurrentlyInteractingWith (Utilities|Array|Get(acopy) _staticspawnfrombackpack_3 (Variables|Default|GetArrayPositionInteractingWith)))))
    (else
      (bind _result_2 (Math|Integer|DecrementInt (Variables|Default|GetArrayPositionInteractingWith))
        (:%20%20
          (if (< _result_2 0)
            (Variables|Default|SetArrayPositionInteractingWith (- _returnvalue 1)))
          (Variables|Default|SetActorCurrentlyInteractingWith (Utilities|Array|Get(acopy) _staticspawnfrombackpack_3 (Variables|Default|GetArrayPositionInteractingWith)))))))
  (if (LocalVariables|GetMovingRight?)
    (for (_array_element _array_index) _staticspawnfrombackpack_2
      (if (< (- _array_index 1) 0)
        (Default|MovetoTransform _array_element (Transformation|GetRelativeTransform (Variables|/Script/Engine.StaticMeshActor|GetStaticMeshComponent (Utilities|Array|Get(acopy) _staticspawnfrombackpack_2 (- (Utilities|Array|Length _staticspawnfrombackpack_2) 1)))))
        (else
          (Default|MovetoTransform _array_element (Transformation|GetRelativeTransform (Variables|/Script/Engine.StaticMeshActor|GetStaticMeshComponent (Utilities|Array|Get(acopy) _staticspawnfrombackpack_2 (- _array_index 1)))))))
      (Default|Selected (Variables|Default|GetActorCurrentlyInteractingWith) (* (CallFunction|GetSpawnSize (Variables|Default|GetActorCurrentlyInteractingWith)) 2.0)))
    (else
      (for (_array_element_2 _array_index_2) _staticspawnfrombackpack
        (if (>= (+ _array_index_2 1) (Utilities|Array|Length _staticspawnfrombackpack))
          (Default|MovetoTransform _array_element_2 (Transformation|GetRelativeTransform (Variables|/Script/Engine.StaticMeshActor|GetStaticMeshComponent (Utilities|Array|Get(acopy) _staticspawnfrombackpack))))
          (else
            (Default|MovetoTransform _array_element_2 (Transformation|GetRelativeTransform (Variables|/Script/Engine.StaticMeshActor|GetStaticMeshComponent (Utilities|Array|Get(acopy) _staticspawnfrombackpack (+ _array_index_2 1)))))))
        (Default|Selected (Variables|Default|GetActorCurrentlyInteractingWith) (* (CallFunction|GetSpawnSize (Variables|Default|GetActorCurrentlyInteractingWith)) 2.0))))))

(fn GetSpawnSize
  (params (Interactable%20Object :type BP%20Interactable%20Object%20Base%20Object%20Reference))
  (bind _staticmeshcomponent (Variables|/Script/Engine.StaticMeshActor|GetStaticMeshComponent Interactable%20Object))
  (bind _staticmesh (Variables|/Script/Engine.StaticMeshComponent|GetStaticMesh _staticmeshcomponent))
  (bind _returnvalue (StaticMesh|GetBoundingBox _staticmesh))
  (bind _returnvalue_2 (Math|Vector|Distance(Vector) (.min _returnvalue) (.max _returnvalue)))
  (bind _returnvalue_3 (/ 4.15 _returnvalue_2))
  (return (Math|Vector|MakeVector _returnvalue_3 _returnvalue_3 _returnvalue_3)))

(fn SelectItem
  (if (Variables|Default|GetBackpackOpen?)
    _))