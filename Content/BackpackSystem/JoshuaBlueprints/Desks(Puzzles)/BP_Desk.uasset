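; BP_Desk is a puzzle desk that defines where specific objects sit on it.
; GetObjectLocationOnDesk switches on the object type (jewellery box, statue, magnifying glass or picture) and returns that object's stored transform variable unchanged.
; Nodes for offsetting the transform by the desk mesh's world transform are left unused, and the event graph and construction script are empty.
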(event EventBeginPlay)

(event Collision|EventActorBeginOverlap
  (params (OtherActor :type Actor%20Object%20Reference)))

(event EventTick
  (params (DeltaSeconds :type Float%20%28single-precision%29)))

(fn ConstructionScript)

(fn GetObjectLocationonDesk
  (params (Object :type ObjectType%20Enum :default "NewEnumerator0"))
  (switch Utilities|FlowControl|Switch|SwitchonObjectType Object
    (:NewEnumerator0
      (return (Variables|Default|GetBoxTransform)))
    (:NewEnumerator1
      (return (Variables|Default|GetStatueTransform)))
    (:NewEnumerator2
      (return (Variables|Default|GetMagGlassTransform)))
    (:NewEnumerator3
      (return (Variables|Default|GetPictureTransform)))))